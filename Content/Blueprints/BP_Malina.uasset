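; BP_Malina is a target actor that halts pheromone-trail laying by overlapping UnitHeroe units and directs ants along the shortest trail.
; On overlap, the hero spawns a pheromone and its spawning timer pauses.
; The ants_start event compares summed trail lengths, then sends all BP_Hive ants along the best one and back via AIMoveTo, advancing on each waypoint's first arrival.
; After the return, it destroys all heroes' pheromones.
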(event Custom|ants_start
  (bind _outactors (Actor|GetAllActorsOfClass "/Game/Units/UnitHeroe.UnitHeroe_C"))
  (for _array_element _outactors
    (for (_array_element_2 _array_index) (Variables|/Game/Units/UnitHeroe.UnitHeroe_C|GetFeromonArray _array_element)
      (if (< (+ _array_index 1) (Utilities|Array|Length (Variables|/Game/Units/UnitHeroe.UnitHeroe_C|GetFeromonArray _array_element)))
        (Variables|Default|Setdistance_sum (+ (Variables|Default|Getdistance_sum) (Transformation|GetDistanceTo _array_element_2 (Utilities|Array|Get(acopy) (Variables|/Game/Units/UnitHeroe.UnitHeroe_C|GetFeromonArray _array_element) (+ _array_index 1)))))))
    (bind _output_get (Variables|Default|Settemp (Variables|Default|Getdistance_sum)))
    (Variables|Default|Setdistance_sum 0.0)
    (if (< _output_get (Variables|Default|Getbest_road))
      (Variables|Default|Setbest_road _output_get)
      (Variables|Default|SetFeromon_array (Variables|/Game/Units/UnitHeroe.UnitHeroe_C|GetFeromonArray _array_element))))
  (bind _returnvalue (Actor|GetActorOfClass "/Game/Blueprints/BP_Hive.BP_Hive_C"))
  (for _array_element_3 (Variables|/Game/Blueprints/BP_Hive.BP_Hive_C|GetAntsArray _returnvalue) :!label _label
    (AI|AIMoveTo (AI|GetAIController _array_element_3) _array_element_3 "0, 0, 0" (Utilities|Array|Get(acopy) (Variables|Default|GetFeromon_array) (Variables|Default|GetIndex)) 5e+01 false
      (:OnSuccess
        (Utilities|FlowControl|DoOnce false
          (:Completed
            (Math|Integer|IncrementInt (Variables|Default|GetIndex)
              (:%20%20
                (if (< (Variables|Default|GetIndex) (Utilities|Array|Length (Variables|Default|GetFeromon_array)))
                  (goto _label)
                  (else
                    (Math|Integer|DecrementInt (Variables|Default|GetIndex)
                      (:%20%20
                        (for _array_element_4 (Variables|/Game/Blueprints/BP_Hive.BP_Hive_C|GetAntsArray _returnvalue) :!label _label_2
                          (AI|AIMoveTo (AI|GetAIController _array_element_4) _array_element_4 "0, 0, 0" (Utilities|Array|Get(acopy) (Variables|Default|GetFeromon_array) (Variables|Default|GetIndex)) 5e+01 false
                            (:OnSuccess
                              (Utilities|FlowControl|DoOnce false
                                (:Completed
                                  (Math|Integer|DecrementInt (Variables|Default|GetIndex)
                                    (:%20%20
                                      (if (>= (Variables|Default|GetIndex) 0)
                                        (goto _label_2)
                                        (else
                                          (bind _outactors_2 (Actor|GetAllActorsOfClass "/Game/Units/UnitHeroe.UnitHeroe_C"))
                                          (for _array_element_5 _outactors_2
                                            (for _array_element_6 (Variables|/Game/Units/UnitHeroe.UnitHeroe_C|GetFeromonArray _array_element_5)
                                              (Actor|DestroyActor _array_element_6)))
                                          (Utilities|Array|Clear (Variables|Default|GetFeromon_array)))))))))))
                        (Utilities|FlowControl|DoOnce false) ; enters at Reset
                      )))))))))))
  (Utilities|FlowControl|DoOnce false) ; enters at Reset
)

(event Collision|EventActorBeginOverlap
  (params (OtherActor :type Actor%20Object%20Reference))
  (bind _asunit_heroe (Utilities|Casting|CastToUnitHeroe OtherActor))
  (Utilities|FlowControl|DoOnce false :!label _label
    (:Completed
      (Default|FeromonSpawn _asunit_heroe)
      (Utilities|Time|PauseTimerbyHandle (Variables|/Game/Units/UnitHeroe.UnitHeroe_C|GetFeromonSpawning _asunit_heroe))
      (goto _label Reset))))

(fn ConstructionScript)