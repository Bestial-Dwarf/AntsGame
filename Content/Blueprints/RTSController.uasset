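; RTS player controller that handles camera zoom, unit selection and move orders.
; The mouse wheel sets the RTSCamera spring arm length, while left press/release starts and stops HUD selection, clearing selected units when the custom-channel trace misses.
; On a similar miss, right click writes the cursor's Visibility hit to each selected unit's Blackboard TargetLocation.
; G calls AntsStart on BP_Malina, and Escape quits the game.
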(event EventBeginPlay
  ;[1 1 1] Inicializacja refa do kamery i game mode'a
  (Input|SetInputModeGameandUI self 0 "LockAlways" false)
  (Utilities|FlowControl|Delay (Utilities|Time|GetWorldDeltaSeconds))
  (bind _asrtscamera (Utilities|Casting|CastToRTSCamera (Pawn|GetViewTarget)))
  (Variables|Default|SetRTSCamera _asrtscamera))

(event Input|MouseEvents|MouseWheelAxis
  (params (AxisValue :type Float%20%28single-precision%29))
  ;[1 1 1] Zoom kamery
  (bind _output_get (Variables|Default|SetZoomFactor (Math|Float|Clamp(Float) (+ (Variables|Default|GetZoomFactor) (* AxisValue -1.0)) 0.0 1e+01)))
  (bind _rtscamera (Variables|Default|GetRTSCamera)
    (:then
      (Variables|/Script/Engine.SpringArmComponent|SetTargetArmLength (Variables|/Game/Blueprints/RTSCamera.RTSCamera_C|GetSpringArm _rtscamera) (+ (* _output_get 2e+02) 1e+03)))
    (:else)))

(event Input|MouseEvents|LeftMouseButton
  (params (Key :type Key%20Structure :default "None"))
  (bind _returnvalue (HUD|GetHUD))
  (:Pressed
    (Class|SelectionInterface|StartSelection(Message) _returnvalue)
    (if (not (.ReturnValue (Game|Player|GetHitResultUnderCursorbyChannel "TraceTypeQuery3" true)))
      (CallFunction|ClearUnitSelection)))
  (:Released
    (Class|SelectionInterface|StopSelection(Message) _returnvalue)))

(event Input|MouseEvents|RightMouseButton
  (params (Key :type Key%20Structure :default "None"))
  (:Pressed
    (if (not (.ReturnValue (Game|Player|GetHitResultUnderCursorbyChannel "TraceTypeQuery3" true)))
      (for _array_element (Variables|Default|GetUnitSelection)
        (AI|Components|Blackboard|SetValueasVector (AI|GetBlackboard _array_element) (Utilities|Name|MakeLiteralName "TargetLocation") (.location (.HitResult (Game|Player|GetHitResultUnderCursorbyChannel "TraceTypeQuery1" true))))))))

(event Input|KeyboardEvents|Escape
  (params (Key :type Key%20Structure :default "None"))
  (:Pressed
    (Game|QuitGame (Class|GameplayStatics|GetPlayerControllerfromID) "Quit" false)))

(event Input|KeyboardEvents|G
  (params (Key :type Key%20Structure :default "None"))
  (:Pressed
    (bind _returnvalue (Actor|GetActorOfClass "/Game/Blueprints/BP_Malina.BP_Malina_C"))
    (Default|AntsStart _returnvalue)))

(fn ConstructionScript)

(fn AddUnittoSelection
  (params (UnitBase :type Unit%20Base%20Object%20Reference))
  (Utilities|Array|AddUnique (Variables|Default|GetUnitSelection) UnitBase)
  (Default|IsSelected UnitBase true))

(fn RemoveUnitfromSelection
  (params (Unit :type Unit%20Base%20Object%20Reference))
  (Utilities|Array|RemoveItem (Variables|Default|GetUnitSelection) Unit)
  (Default|IsSelected Unit false))

(fn ClearUnitSelection
  (for _array_element (Variables|Default|GetUnitSelection)
    (Default|IsSelected _array_element false))
  (Utilities|Array|Clear (Variables|Default|GetUnitSelection)))