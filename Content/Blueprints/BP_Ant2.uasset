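; BP_Ant2 is a selectable ant unit for an RTS-style game.
; A left click casts the player controller to RTSController and adds the unit to the selection, or removes it if already selected.
; The IsSelected event shows or hides a Decal, whose visibility also serves as the selection state checked on click.
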(event Custom|IsSelected
  (params (IsSelected :type Boolean))
  (Rendering|SetVisibility (Variables|Default|GetDecal) IsSelected false))

(event MouseInput|EventActorOnClicked
  (params (ButtonPressed :type Key%20Structure :default "None"))
  (if (== ButtonPressed "LeftMouseButton")
    (bind _asrtscontroller (Utilities|Casting|CastToRTSController (Game|GetPlayerController 0)))
    (if (Rendering|IsVisible (Variables|Default|GetDecal))
      (Default|RemoveUnitfromSelection _asrtscontroller)
      (else
        (Default|AddUnittoSelection _asrtscontroller)))))

(fn ConstructionScript)